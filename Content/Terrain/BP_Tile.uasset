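; Endless-terrain tile that scatters props, rocks and AI characters on BeginPlay and exposes its Arrow transform as an attach point.
; Its barrier starts locked, turning green and passable when the player enters LockingVolume from below the Arrow's X.
; Exiting beyond that X relocks it red and reports a conquered tile to the game mode.
; Player overlap with DestructionVolume asks the game mode for another tile, then destroys this one.
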(event `self.ReceiveBeginPlay`
  (`self.Lock`)
  (`self.PlaceActors` "/Game/Terrain/Props/BP_Container.BP_Container_C" 1 3 225.0)
  (`self.PlaceActors` "/Game/Terrain/Props/BP_Box.BP_Box_C" 2 5 70.0)
  (`self.PlaceActors` "/Game/Terrain/Props/BP_Cannister.BP_Cannister_C" 1 4 35.0)
  (`self.PlaceActors` "/Game/Terrain/Props/BP_Rock01.BP_Rock01_C" 1 3 125.0 4.0)
  (`self.PlaceActors` "/Game/Terrain/Props/BP_Rock05.BP_Rock05_C" 1 3 200.0 4.0)
  (`self.PlaceActors` "/Game/Terrain/Props/BP_Rock17.BP_Rock17_C" 1 3 200.0 4.0)
  (`self.PlaceActors` "/Game/Terrain/Props/BP_Sackwall.BP_Sackwall_C" 1 3 325.0)
  (`self.PlaceAIPawns` "/Game/Character/Behavior/BP_Character.BP_Character_C" 2 4 40.0))

(event `self.Locking Volume.OnComponentBeginOverlap`
  (params (OverlappedComponent :type "PrimitiveComponent Object Reference") (OtherActor :type "Actor Object Reference") (OtherComp :type "PrimitiveComponent Object Reference") (OtherBodyIndex :type Integer) (bFromSweep :type Boolean) (SweepResult :type "HitResult Structure (by ref)"))
  (bind _returnvalue_x (`KismetMathLibrary.BreakVector` (`self.K2_GetActorLocation` OtherActor)))
  (bind _returnvalue_x_2 (`KismetMathLibrary.BreakVector` (`SceneComponent.K2_GetComponentLocation` (`self.Arrow`))))
  (`self.Is Player Actor` OtherActor)
  (if (< _returnvalue_x _returnvalue_x_2)
    (`self.Unlock`)))

(event `self.Locking Volume.OnComponentEndOverlap`
  (params (OverlappedComponent :type "PrimitiveComponent Object Reference") (OtherActor :type "Actor Object Reference") (OtherComp :type "PrimitiveComponent Object Reference") (OtherBodyIndex :type Integer))
  (bind _returnvalue_x (`KismetMathLibrary.BreakVector` (`self.K2_GetActorLocation` OtherActor)))
  (bind _returnvalue_x_2 (`KismetMathLibrary.BreakVector` (`SceneComponent.K2_GetComponentLocation` (`self.Arrow`))))
  (`self.Is Player Actor` OtherActor)
  (if (> _returnvalue_x _returnvalue_x_2)
    (`self.Lock`)
    (bind _asbp_infinite_terrain_game_mode (cast `/Game/Blueprints/BP_InfiniteTerrainGameMode` (`GameplayStatics.GetGameMode`)))
    (`InfiniteTerrainGameMode.NewTileConquered` _asbp_infinite_terrain_game_mode)))

(event `self.Destruction Volume.OnComponentBeginOverlap`
  (params (OverlappedComponent :type "PrimitiveComponent Object Reference") (OtherActor :type "Actor Object Reference") (OtherComp :type "PrimitiveComponent Object Reference") (OtherBodyIndex :type Integer) (bFromSweep :type Boolean) (SweepResult :type "HitResult Structure (by ref)"))
  (`self.Is Player Actor` OtherActor)
  (bind _asbp_infinite_terrain_game_mode (cast `/Game/Blueprints/BP_InfiniteTerrainGameMode` (`GameplayStatics.GetGameMode`)))
  (`/Game/Blueprints/BP_InfiniteTerrainGameMode.Spawn Tile` _asbp_infinite_terrain_game_mode)
  (`self.K2_DestroyActor`))

(fn `Get Attach Location`
  (returns (`Attach Transform` :type "Transform Structure"))
  (return (`SceneComponent.K2_GetComponentToWorld` (`self.Arrow`))))

(fn `Lock`
  (`PrimitiveComponent.SetCollisionEnabled` (`self.Barrier`) "QueryAndPhysics")
  (`PrimitiveComponent.SetMaterial` (`self.Barrier`) 0 "/Game/Geometry/Meshes/RedBarrier.RedBarrier"))

(fn `Unlock`
  (`PrimitiveComponent.SetCollisionEnabled` (`self.Barrier`) "NoCollision")
  (`PrimitiveComponent.SetMaterial` (`self.Barrier`) 0 "/Game/Geometry/Meshes/GreenBarrier.GreenBarrier"))

(fn `UserConstructionScript`)